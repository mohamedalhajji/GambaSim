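; BP_Chair is a card-table seat that detects the player and moves them into and out of it.
; Box overlap shows a prompt widget above the chair and enables input, and leaving removes the widget.
; Sit and Stand events, not called here, use timelines to lerp-teleport the character onto the Cylinder or to an offset beside it.
; Sitting ends in UI-only input focused on BP_DeckManager's HUD, and standing restores game-only input.
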(event OnComponentBeginOverlap(Box)
  (params (OverlappedComponent :type Primitive%20Component%20Object%20Reference) (OtherActor :type Actor%20Object%20Reference) (OtherComp :type Primitive%20Component%20Object%20Reference) (OtherBodyIndex :type Integer) (bFromSweep :type Boolean) (SweepResult :type Hit%20Result%20Structure%20%28by%20ref%29))
  ;[0 0 0 1 25] Chair Detection
  (bind _returnvalue (AddComponent|AddWidgetComponent false (Math|Transform|MakeTransform "0.000000,0.000000,70.000000" "0, 0, 0" "1.000000,1.000000,1.000000")))
  (Variables|Default|SetChairHUDWD _returnvalue)
  (Input|EnableInput (Game|GetPlayerController 0)) ; needed for E
  (Variables|Default|SetIsOverlapping true))

(event OnComponentEndOverlap(Box)
  (params (OverlappedComponent :type Primitive%20Component%20Object%20Reference) (OtherActor :type Actor%20Object%20Reference) (OtherComp :type Primitive%20Component%20Object%20Reference) (OtherBodyIndex :type Integer))
  ;[0 0 0 1 25] Chair Detection
  (if (Variables|Default|GetIsOverlapping)
    (Components|DestroyComponent (Variables|Default|GetChairHUDWD))
    (Variables|Default|SetIsOverlapping false)))

(event Custom|Stand
  (bind _cylinder (Variables|Default|GetCylinder))
  (bind _returnvalue (Transformation|GetWorldLocation _cylinder))
  (bind (_x _y _z) (Math|Vector|BreakVector _returnvalue))
  ;[0 0 0 1 25] Sitting & Standing Fucntions
  (bind _standing (Timeline|Timeline_0 PlayFromStart)
    (:Update
      (Transformation|SetActorLocation (Game|GetPlayerCharacter 0) (Math|Vector|Lerp(Vector) (Transformation|GetActorLocation (Game|GetPlayerCharacter 0)) (Math|Transform|TransformLocation (Math|Transform|MakeTransform "-100.000000,0.000000,0.000000" "0, 0, 0" "1.000000,1.000000,1.000000") (Math|Vector|MakeVector _x _y (+ _z 98.213))) _standing) false true))
    (:Finished
      (Input|SetInputModeGameOnly (Game|GetPlayerController 0) false))))

(event Custom|Sit
  (bind _cylinder (Variables|Default|GetCylinder))
  (bind _returnvalue (Transformation|GetWorldLocation _cylinder))
  (bind (_x _y _z) (Math|Vector|BreakVector _returnvalue))
  ;[0 0 0 1 25] Sitting & Standing Fucntions
  (bind _sitting (Timeline|Timeline PlayFromStart)
    (:Update
      (Transformation|SetActorLocation (Game|GetPlayerCharacter 0) (Math|Vector|Lerp(Vector) (Transformation|GetActorLocation (Game|GetPlayerCharacter 0)) (Math|Vector|MakeVector _x _y (+ _z 98.213)) _sitting) false true))
    (:Finished
      (Input|SetInputModeUIOnly (Game|GetPlayerController 0) (Variables|/Game/Main/Blueprints/BP_DeckManager.BP_DeckManager_C|GetWD%20BJHUD%20Ref (Variables|Default|GetDM%20Ref)) "DoNotLock" false))))

(event EventBeginPlay
  (Utilities|FlowControl|Delay 0.2)
  (bind _returnvalue (Actor|GetActorOfClass "/Game/Main/Blueprints/BP_DeckManager.BP_DeckManager_C"))
  (Variables|Default|SetDM%20Ref _returnvalue))

(fn ConstructionScript)