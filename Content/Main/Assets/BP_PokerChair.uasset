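; BP_PokerChair is an interactable chair that switches the player to an overhead poker view with its own HUD.
; Interact while overlapping calls Sit, then Camera shows the PokerHUD created at BeginPlay, enables the cursor and blends to a spawned, downward-facing BP_Camera at a hardcoded world position.
; Uncamera removes the HUD, blends back to the character, destroys the camera after the blend and restores game-only input.
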(event Custom|Uncamera
  (bind _returnvalue (Game|GetPlayerController 0))
  (Widget|RemovefromParent (Variables|Default|GetPokerWD))
  (Game|Player|SetViewTargetwithBlend (Game|GetPlayerController 0) (Game|GetPlayerCharacter 0) 0.5 "VTBlend_EaseInOut" 3.0 false)
  (Utilities|FlowControl|Delay 0.5)
  (Actor|DestroyActor (Variables|Default|GetCamRef))
  (Variables|/Script/Engine.PlayerController|SetbShowMouseCursor _returnvalue false)
  (Input|SetInputModeGameOnly _returnvalue false))

(event Input|EnhancedActionEvents|EnhancedInputActionInteract
  (params (ActionValue :type Boolean) (ElapsedSeconds :type Float%20%28double-precision%29) (TriggeredSeconds :type Float%20%28double-precision%29) (InputAction :type Input%20Action%20Object%20Reference :default "/Game/Main/Input/Actions/Key_Presses/Interact.Interact"))
  ;[0 0 0 1 25] Bar Func
  (:Started
    (if (Variables|Default|GetIsOverlapping)
      (CallFunction|Sit)
      (CallFunction|Camera))))

(event EventBeginPlay
  (bind _returnvalue (UserInterface|CreateWidget "/Game/Main/UI/Widgets/Gameplay/Poker/PokerHUD.PokerHUD_C"))
  (Variables|Default|SetPokerWD _returnvalue))

(fn ConstructionScript
  (|CallParentFunction))

(fn Camera
  (bind _returnvalue (Game|GetPlayerController 0))
  (bind _pokerwd (Variables|Default|GetPokerWD))
  (UserInterface|Viewport|AddtoViewport _pokerwd 1)
  (Input|SetInputModeGameandUI _returnvalue _pokerwd "DoNotLock" true false)
  (Variables|/Script/Engine.PlayerController|SetbShowMouseCursor _returnvalue true)
  (bind _returnvalue_2 (Game|SpawnActorfromClass "/Game/Main/Assets/BP_Camera.BP_Camera_C" (Math|Transform|MakeTransform "230.000000,-880.000000,500.000000" "-89.000000,0.000000,0.000000" "1.000000,1.000000,1.000000") "AlwaysSpawn" "MultiplyWithRoot" 0 0))
  (bind _output_get (Variables|Default|SetCamRef _returnvalue_2))
  (Game|Player|SetViewTargetwithBlend (Game|GetPlayerController 0) _output_get 1.0 "VTBlend_EaseInOut" 3.0 false))