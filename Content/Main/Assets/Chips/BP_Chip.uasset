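; BP_Chip is a casino-style chip actor whose appearance depends on its ChipValue denomination.
; The construction script calls SetMaterial, which switches on ChipValue to assign the matching chip material to slot 0 of the static mesh.
; On BeginPlay it waits briefly, then caches a reference to BP_DeckManager, retrying once after another short delay if none is found.
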(event EventBeginPlay
  (Utilities|FlowControl|Delay 0.2)
  (bind _returnvalue (Actor|GetActorOfClass "/Game/Main/Blueprints/BP_DeckManager.BP_DeckManager_C"))
  (bind _output_get (Variables|Default|SetDM%20Ref _returnvalue))
  (Utilities|IsValid _output_get
    (:Is%20Not%20Valid
      (Utilities|FlowControl|Delay 0.2)
      (bind _returnvalue_2 (Actor|GetActorOfClass "/Game/Main/Blueprints/BP_DeckManager.BP_DeckManager_C"))
      (Variables|Default|SetDM%20Ref _returnvalue_2))))

(fn ConstructionScript
  (CallFunction|SetMaterial))

(fn SetMaterial
  (bind _staticmesh (Variables|Default|GetStaticMesh))
  (switch Utilities|FlowControl|Switch|SwitchonE_ChipValue (Variables|Default|GetChip%20Value)
    (:NewEnumerator0
      (Rendering|Material|SetMaterial _staticmesh 0 "/Game/Main/Assets/Chips/M_Chip_1.M_Chip_1"))
    (:NewEnumerator1
      (Rendering|Material|SetMaterial _staticmesh 0 "/Game/Main/Assets/Chips/M_Chip_5.M_Chip_5"))
    (:NewEnumerator2
      (Rendering|Material|SetMaterial _staticmesh 0 "/Game/Main/Assets/Chips/M_Chip_10.M_Chip_10"))
    (:NewEnumerator3
      (Rendering|Material|SetMaterial _staticmesh 0 "/Game/Main/Assets/Chips/M_Chip_50.M_Chip_50"))
    (:NewEnumerator4
      (Rendering|Material|SetMaterial _staticmesh 0 "/Game/Main/Assets/Chips/M_Chip_100.M_Chip_100"))
    (:NewEnumerator5
      (Rendering|Material|SetMaterial _staticmesh 0 "/Game/Main/Assets/Chips/M_Chip_500.M_Chip_500"))
    (:NewEnumerator6
      (Rendering|Material|SetMaterial _staticmesh 0 "/Game/Main/Assets/Chips/M_Chip_1000.M_Chip_1000"))))