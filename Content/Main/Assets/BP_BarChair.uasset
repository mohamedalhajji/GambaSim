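; BP_BarChair is an interactable bar seat that opens the bar UI when the player interacts while overlapping it.
; Interacting calls Sit, shows the bar widget held by BP_DeckManager, enables the cursor, and blends the view to a BP_Camera spawned at a hard-coded location.
; Uncamera removes the widget, blends back to the character, destroys the camera, and restores game-only input.
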(event Custom|Uncamera
  (bind _returnvalue (Game|GetPlayerController 0))
  (Widget|RemovefromParent (Variables|/Game/Main/Blueprints/BP_DeckManager.BP_DeckManager_C|GetWD%20Bar%20Ref (Variables|Default|GetDM%20Ref)))
  (Game|Player|SetViewTargetwithBlend (Game|GetPlayerController 0) (Game|GetPlayerCharacter 0) 0.5 "VTBlend_EaseInOut" 3.0 false)
  (Utilities|FlowControl|Delay 0.5)
  (Actor|DestroyActor (Variables|Default|GetCamRef))
  (Variables|/Script/Engine.PlayerController|SetbShowMouseCursor _returnvalue false)
  (Input|SetInputModeGameOnly _returnvalue false))

(event Input|EnhancedActionEvents|EnhancedInputActionInteract
  (params (ActionValue :type Boolean) (ElapsedSeconds :type Float%20%28double-precision%29) (TriggeredSeconds :type Float%20%28double-precision%29) (InputAction :type Input%20Action%20Object%20Reference :default "/Game/Main/Input/Actions/Interact.Interact"))
  ;[0 0 0 1 25] Bar Func
  (:Started
    (if (Variables|Default|GetIsOverlapping)
      (CallFunction|Sit)
      (CallFunction|Camera))))

(event EventBeginPlay
  (Utilities|FlowControl|Delay 0.2)
  (bind _returnvalue (Actor|GetActorOfClass "/Game/Main/Blueprints/BP_DeckManager.BP_DeckManager_C"))
  (Variables|Default|SetDM%20Ref _returnvalue))

(fn ConstructionScript
  (|CallParentFunction))

(fn Camera
  (bind _returnvalue (Game|GetPlayerController 0))
  (UserInterface|Viewport|AddtoViewport (Variables|/Game/Main/Blueprints/BP_DeckManager.BP_DeckManager_C|GetWD%20Bar%20Ref (Variables|Default|GetDM%20Ref)) 1)
  (Input|SetInputModeGameandUI _returnvalue 0 "DoNotLock" false false)
  (Variables|/Script/Engine.PlayerController|SetbShowMouseCursor _returnvalue true)
  (bind _returnvalue_2 (Game|SpawnActorfromClass "/Game/Main/Assets/BP_Camera.BP_Camera_C" (Math|Transform|MakeTransform "1050.000000,-50.000000,160.000000" "0, 0, 0" "1.000000,1.000000,1.000000") "Undefined" "MultiplyWithRoot" 0 0))
  (bind _output_get (Variables|Default|SetCamRef _returnvalue_2))
  (Game|Player|SetViewTargetwithBlend (Game|GetPlayerController 0) _output_get 0.5 "VTBlend_EaseInOut" 3.0 false))