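; BP_BJChair is a chair that seats the player at a blackjack game when they press Interact while overlapping it.
; Interacting sits the player, switches to UI input, blends the view to a spawned camera, and plays a loading animation.
; When that animation finishes, it calls StopGame on the cached BP_DeckManager and shows its HUD.
; Uncamera removes the HUD, blends back to the character, destroys the camera and restores game input.
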(event Custom|Uncamera
  (bind _returnvalue (Game|GetPlayerController 0))
  (Utilities|DMRefCheck
    (:Exec%20Out
      (Widget|RemovefromParent (Variables|/Game/Main/Blueprints/BP_DeckManager.BP_DeckManager_C|GetWD%20BJHUD%20Ref (Variables|Default|GetDM%20Ref)))
      (Game|Player|SetViewTargetwithBlend (Game|GetPlayerController 0) (Game|GetPlayerCharacter 0) 0.5 "VTBlend_EaseInOut" 3.0 false)
      (Utilities|FlowControl|Delay 0.5)
      (Actor|DestroyActor (Variables|Default|GetCamRef))
      (Variables|/Script/Engine.PlayerController|SetbShowMouseCursor _returnvalue false)
      (Input|SetInputModeGameOnly _returnvalue false))))

(event Input|EnhancedActionEvents|EnhancedInputActionInteract
  (params (ActionValue :type Boolean) (ElapsedSeconds :type Float%20%28double-precision%29) (TriggeredSeconds :type Float%20%28double-precision%29) (InputAction :type Input%20Action%20Object%20Reference :default "/Game/Main/Input/Actions/Key_Presses/Interact.Interact"))
  (bind _bjloading_wd (Variables|Default|GetBJLoading%20WD))
  (bind _dm_ref (Variables|Default|GetDM%20Ref))
  ;[0 0 0 1 25] BJ Func
  (:Started
    (if (Variables|Default|GetIsOverlapping)
      (Utilities|DMRefCheck
        (:Exec%20Out
          (CallFunction|Sit)
          (CallFunction|Camera)
          (UserInterface|Viewport|AddtoViewport _bjloading_wd 0)
          (Components|Animation|PlayAnimation _bjloading_wd (Variables|/Game/Main/UI/Widgets/Gameplay/BJ/WD_BJLoading.WD_BJLoading_C|GetLoading_Text _bjloading_wd) 0.0
            (:Finished
              (Default|StopGame _dm_ref)
              (UserInterface|Viewport|AddtoViewport (Variables|/Game/Main/Blueprints/BP_DeckManager.BP_DeckManager_C|GetWD%20BJHUD%20Ref _dm_ref) 0))))))))

(event EventBeginPlay
  (Utilities|FlowControl|Delay 0.2)
  (bind _returnvalue (UserInterface|CreateWidget "/Game/Main/UI/Widgets/Gameplay/BJ/WD_BJLoading.WD_BJLoading_C"))
  (Variables|Default|SetBJLoading%20WD _returnvalue)
  (bind _returnvalue_2 (Actor|GetActorOfClass "/Game/Main/Blueprints/BP_DeckManager.BP_DeckManager_C"))
  (Variables|Default|SetDM%20Ref _returnvalue_2))

(fn ConstructionScript
  (|CallParentFunction))

(fn Camera
  (bind _returnvalue (Game|GetPlayerController 0))
  (Input|SetInputModeUIOnly _returnvalue (Variables|/Game/Main/Blueprints/BP_DeckManager.BP_DeckManager_C|GetWD%20BJHUD%20Ref (Variables|Default|GetDM%20Ref)) "DoNotLock" false)
  (Variables|/Script/Engine.PlayerController|SetbShowMouseCursor _returnvalue true)
  (bind _returnvalue_2 (Game|SpawnActorfromClass "/Game/Main/Assets/BP_Camera.BP_Camera_C" (Math|Transform|MakeTransform (Math|Vector|MakeVector 1e+02 8e+02 2.5e+02) "-50.000000,0.000000,0.000000" "1.000000,1.000000,1.000000") "AlwaysSpawn" "MultiplyWithRoot" 0 0))
  (bind _output_get (Variables|Default|SetCamRef _returnvalue_2))
  (Game|Player|SetViewTargetwithBlend (Game|GetPlayerController 0) _output_get 0.5 "VTBlend_EaseInOut" 3.0 false))