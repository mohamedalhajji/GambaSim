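; Interactive prize wheel the player spins by dragging the mouse.
; After a character overlaps its box, Interact toggles a blend to a spawned fixed-position camera, with cursor and IMC_Wheel mapping context.
; Held-mouse movement rolls the wheel, using the cursor's screen quadrant to sign the spin.
; A strong enough positive spin locks dragging and picks one of twelve random results, then a Timeline lerps through several turns to that preset angle.
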(event OnComponentBeginOverlap(Box)
  (params (OverlappedComponent :type Primitive%20Component%20Object%20Reference) (OtherActor :type Actor%20Object%20Reference) (OtherComp :type Primitive%20Component%20Object%20Reference) (OtherBodyIndex :type Integer) (bFromSweep :type Boolean) (SweepResult :type Hit%20Result%20Structure%20%28by%20ref%29))
  (bind _asbp_first_person_character (Utilities|Casting|CastToBP_FirstPersonCharacter OtherActor)))

(event Input|EnhancedActionEvents|EnhancedInputActionInteract
  (params (ActionValue :type Boolean) (ElapsedSeconds :type Float%20%28double-precision%29) (TriggeredSeconds :type Float%20%28double-precision%29) (InputAction :type Input%20Action%20Object%20Reference :default "/Game/Main/Input/Actions/Key_Presses/Interact.Interact"))
  (bind _returnvalue (Game|GetPlayerController 0))
  (bind _returnvalue_2 (Game|GetPlayerController 0))
  (bind _returnvalue_3 (Game|GetPlayerController 0))
  (bind _returnvalue_4 (PlayerController|LocalPlayerSubsystems|GetEnhancedInputLocalPlayerSubsystem _returnvalue))
  (:Started
    (Utilities|FlowControl|DoOnce false :!label _label
      (:Completed
        (if (Variables|Default|GetIsInteracted)
          (Variables|/Script/Engine.PlayerController|SetbShowMouseCursor _returnvalue_3 false)
          (Game|Player|SetViewTargetwithBlend _returnvalue_3 (Game|GetPlayerCharacter 0) 0.5 "VTBlend_EaseInOut" 3.0 false)
          (Utilities|FlowControl|Delay 0.5)
          (Actor|DestroyActor (stale _returnvalue_5))
          (Input|RemoveMappingContext _returnvalue_4 "/Game/Main/Input/IMC_Wheel.IMC_Wheel" "(bIgnoreAllPressedKeysUntilRelease=True,bForceImmediately=False,bNotifyUserSettings=False)")
          (Variables|Default|SetIsInteracted false)
          (goto _label Reset)
          (else
            (Utilities|IsValid (stale OnComponentBeginOverlap(Box) _asbp_first_person_character)
              (:Is%20Valid
                (Variables|Default|SetIsInteracted true)
                (Variables|/Script/Engine.PlayerController|SetbShowMouseCursor _returnvalue_2 true)
                (bind _returnvalue_5 (Game|SpawnActorfromClass "/Game/Main/Assets/BP_Camera.BP_Camera_C" (Math|Transform|MakeTransform "1370.000000,785.000000,170.000000" "0, 0, 0" "1.000000,1.000000,1.000000") "Undefined" "MultiplyWithRoot" 0 0))
                (Game|Player|SetViewTargetwithBlend _returnvalue_2 _returnvalue_5 0.5 "VTBlend_EaseInOut" 3.0 false)
                (Input|AddMappingContext _returnvalue_4 "/Game/Main/Input/IMC_Wheel.IMC_Wheel" 1 "(bIgnoreAllPressedKeysUntilRelease=True,bForceImmediately=False,bNotifyUserSettings=False)")
                (Utilities|FlowControl|Delay 0.5)
                (goto _label Reset)))))))))

(event Input|EnhancedActionEvents|EnhancedInputActionWheel
  (params (ActionValue :type Vector%202D%20Structure) (ElapsedSeconds :type Float%20%28double-precision%29) (TriggeredSeconds :type Float%20%28double-precision%29) (InputAction :type Input%20Action%20Object%20Reference :default "/Game/Main/Input/Actions/Movement/Wheel.Wheel"))
  (bind _returnvalue (Viewport|GetViewportSize))
  (bind _scene (Variables|Default|GetScene))
  (bind _returnvalue_2 (/ _returnvalue 2.0))
  (if (Math|Boolean|ANDBoolean (Variables|Default|GetIsM1) (Variables|Default|GetIsInteracted) (not (Variables|Default|GetIsStrong)))
    (bind _returnvalue_3 (Class|WidgetLayoutLibrary|GetMousePositiononPlatform))
    (if (and (>= (.x _returnvalue_3) (.x _returnvalue_2)) (>= (.y _returnvalue_3) (.y _returnvalue_2)))
      (bind _output_get (Variables|Default|SetSpin%20Power (* (+ (.x ActionValue) (.y ActionValue)) 0.75)))
      (Transformation|AddWorldRotation _scene (Math|Rotator|MakeRotator _output_get 0.0 0.0) false false) ; Bottom Right
      (elif (>= (.x _returnvalue_3) (.x _returnvalue_2))
        (bind _output_get_2 (Variables|Default|SetSpin%20Power (+ (.y ActionValue) (* (.x ActionValue) -0.75))))
        (Transformation|AddWorldRotation _scene (Math|Rotator|MakeRotator _output_get_2 0.0 0.0) false false) ; Top RIght
        (elif (>= (.y _returnvalue_3) (.y _returnvalue_2))
          (bind _output_get_3 (Variables|Default|SetSpin%20Power (+ (.x ActionValue) (* (.y ActionValue) -0.75))))
          (Transformation|AddWorldRotation _scene (Math|Rotator|MakeRotator _output_get_3 0.0 0.0) false false) ; Bottom Left
          (else
            (bind _output_get_4 (Variables|Default|SetSpin%20Power (* (+ (.x ActionValue) (.y ActionValue)) -0.75)))
            (Transformation|AddWorldRotation _scene (Math|Rotator|MakeRotator _output_get_4 0.0 0.0) false false) ; Top Left
          ))))
    (if (> (Variables|Default|GetSpin%20Power) 7.0)
      (Utilities|FlowControl|Delay 0.01)
      (if (Input|EnhancedActionValues|GetMouse_One)
        (Utilities|FlowControl|DoOnce false :!label _label
          (:Completed
            (Variables|Default|SetIsStrong true)
            (Variables|Default|SetOG (Variables|/Script/Engine.SceneComponent|GetRelativeRotation (Variables|Default|GetScene)))
            (bind _output_get_5 (Variables|Default|SetPrize (Math|Random|RandomIntegerinRange 0 11)))
            (switch int _output_get_5
              (:0
                (Variables|Default|SetDest "0.000000,0.000000,-15.000000")
                (bind _newtrack_0 (Timeline|Timeline PlayFromStart)
                  (:Update
                    (Transformation|SetRelativeRotation (Variables|Default|GetScene) (Math|Rotator|Lerp(Rotator) (Variables|Default|GetOG) (Math|Rotator|MakeRotator (+ (* 3.6e+02 -5.0) (.roll (Variables|Default|GetDest))) (.pitch (Variables|Default|GetDest)) (.yaw (Variables|Default|GetDest))) _newtrack_0) false false))
                  (:Finished
                    (Variables|Default|SetIsStrong false)
                    (goto _label Reset))))
              (:1
                (Variables|Default|SetDest "0.000000,0.000000,10.000000")
                (Timeline|Timeline PlayFromStart))
              (:2
                (Variables|Default|SetDest "0.000000,0.000000,55.000000")
                (Timeline|Timeline PlayFromStart))
              (:3
                (Variables|Default|SetDest "0.000000,0.000000,87.000000")
                (Timeline|Timeline PlayFromStart))
              (:4
                (Variables|Default|SetDest "0.000000,0.000000,100.000000")
                (Timeline|Timeline PlayFromStart))
              (:5
                (Variables|Default|SetDest "0.000000,0.000000,125.000000")
                (Timeline|Timeline PlayFromStart))
              (:6
                (Variables|Default|SetDest "0.000000,0.000000,165.000000")
                (Timeline|Timeline PlayFromStart))
              (:7
                (Variables|Default|SetDest "0.000000,0.000000,200.000000")
                (Timeline|Timeline PlayFromStart))
              (:8
                (Variables|Default|SetDest "0.000000,0.000000,220.000000")
                (Timeline|Timeline PlayFromStart))
              (:9
                (Variables|Default|SetDest "0.000000,0.000000,243.000000")
                (Timeline|Timeline PlayFromStart))
              (:10
                (Variables|Default|SetDest "0.000000,0.000000,272.000000")
                (Timeline|Timeline PlayFromStart))
              (:11
                (Variables|Default|SetDest "0.000000,0.000000,325.000000")
                (Timeline|Timeline PlayFromStart)))))
        (else
          (goto _label Reset)))
      (else
        (goto _label Reset)))))

(event Input|EnhancedActionEvents|EnhancedInputActionMouse_One
  (params (ActionValue :type Boolean) (ElapsedSeconds :type Float%20%28double-precision%29) (TriggeredSeconds :type Float%20%28double-precision%29) (InputAction :type Input%20Action%20Object%20Reference :default "/Game/Main/Input/Actions/Movement/Mouse_One.Mouse_One"))
  (:Triggered
    (Variables|Default|SetIsM1 true :!label _label))
  (:Started
    (goto _label))
  (:Ongoing
    (goto _label))
  (:Canceled
    (Variables|Default|SetIsM1 false :!label _label_2))
  (:Completed
    (goto _label_2)))

(event EventBeginPlay
  (Input|EnableInput (Game|GetPlayerController 0)))

(fn ConstructionScript)