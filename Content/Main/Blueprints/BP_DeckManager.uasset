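; BP_DeckManager manages the card deck and round reset for the blackjack minigame.
; BeginPlay creates the blackjack, results and bar menu widgets and caches references to the table, chair, stats manager and game instance.
; InitializeCards builds the deck from every value and suit pair, shuffling after each addition.
; Reset clears the deck and restores HUD split and double flags, optionally the bet; StopGame always resets the bet.
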(event EventBeginPlay
  ;[0 0 0] Ref Gets
  (bind _returnvalue (UserInterface|CreateWidget "/Game/Main/UI/Widgets/Gameplay/BJ/WD_BJ.WD_BJ_C"))
  (Variables|Refs|SetWD%20BJHUD%20Ref _returnvalue)
  (bind _returnvalue_2 (Actor|GetActorOfClass "/Game/Main/Blueprints/BP_StatsManager.BP_StatsManager_C"))
  (Variables|Refs|SetCalcMGR%20Ref _returnvalue_2)
  (bind _asmy_game_instance (Utilities|Casting|CastToMyGameInstance (Game|GetGameInstance)))
  (Variables|Refs|SetStats%20Ref _asmy_game_instance)
  (bind _returnvalue_3 (UserInterface|CreateWidget "/Game/Main/UI/Widgets/Gameplay/BJ/WD_BJResults.WD_BJResults_C"))
  (Variables|Refs|SetWD%20Results%20Ref _returnvalue_3)
  (bind _returnvalue_4 (Actor|GetActorOfClass "/Game/Main/Assets/BP_BJChair.BP_BJChair_C"))
  (Variables|Refs|SetBJChair%20Ref _returnvalue_4)
  (bind _returnvalue_5 (UserInterface|CreateWidget "/Game/Main/UI/Widgets/Gameplay/Bar/BarDrinkMenu.BarDrinkMenu_C"))
  (Variables|Refs|SetWD%20Bar%20Ref _returnvalue_5)
  (bind _returnvalue_6 (Actor|GetActorOfClass "/Game/Main/Blueprints/BP_Blackjack.BP_Blackjack_C"))
  (Variables|Refs|SetBJ%20Ref _returnvalue_6))

(fn ConstructionScript)

(fn InitializeCards
  (bind _deck (Variables|MainVars|GetDeck))
  (bind _enumvalue (|ForEachE_CardValues)
    (:LoopBody
      (bind _enumvalue_2 (|ForEachE_CardSuits)
        (:LoopBody
          (Utilities|Array|Add _deck (Utilities|Struct|MakeS_Cards _enumvalue _enumvalue_2))
          (Utilities|Array|Shuffle _deck))))))

(fn StopGame
  (Utilities|Reset true))