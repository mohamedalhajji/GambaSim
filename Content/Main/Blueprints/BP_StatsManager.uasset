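; Blackjack stats manager that settles hand results into money and XP.
; Calc branches on split and double-down states, pays wins and pushes through MoneySum, triggers XPReward and shows results.
; XPReward picks normal, 21 or double-21 rewards; XPSum adds half the bet, dividing the new XP total by BKcon when bankrupted, then saves.
; BeginPlay caches BP_DeckManager, the hub for game references, and loads the bankruptcy flag from the "BK" save slot.
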(event EventBeginPlay
  (Utilities|FlowControl|Delay 0.1)
  (bind _returnvalue (Actor|GetActorOfClass "/Game/Main/Blueprints/BP_DeckManager.BP_DeckManager_C"))
  (Variables|Default|SetDM%20ref _returnvalue)
  (CallFunction|SettingBK))

(fn ConstructionScript)

(fn Calc
  (params (Calc :type E_Calc%20Enum :default "NewEnumerator0") (SP1_Calc :type E_Calc%20Enum :default "NewEnumerator0") (SP2_Calc :type E_Calc%20Enum :default "NewEnumerator0"))
  (bind _dm_ref (Variables|Default|GetDM%20ref))
  (bind _dm_ref_2 (Variables|Default|GetDM%20ref))
  (bind _dm_ref_3 (Variables|Default|GetDM%20ref))
  (bind _dm_ref_4 (Variables|Default|GetDM%20ref))
  (bind _wd_bjhud_ref (Variables|/Game/Main/Blueprints/BP_DeckManager.BP_DeckManager_C|GetWD%20BJHUD%20Ref _dm_ref_4))
  (bind _wd_bjhud_ref_2 (Variables|/Game/Main/Blueprints/BP_DeckManager.BP_DeckManager_C|GetWD%20BJHUD%20Ref _dm_ref))
  (bind _bj_ref (Variables|/Game/Main/Blueprints/BP_DeckManager.BP_DeckManager_C|GetBJ%20Ref _dm_ref_3))
  (bind _bj_ref_2 (Variables|/Game/Main/Blueprints/BP_DeckManager.BP_DeckManager_C|GetBJ%20Ref _dm_ref_2))
  (bind _betamount (Variables|/Game/Main/UI/Widgets/Gameplay/BJ/WD_BJ.WD_BJ_C|GetBetAmount _wd_bjhud_ref_2))
  (bind _betamount_2 (Variables|/Game/Main/UI/Widgets/Gameplay/BJ/WD_BJ.WD_BJ_C|GetBetAmount _wd_bjhud_ref))
  (bind _sp1_bet_amount (Variables|/Game/Main/UI/Widgets/Gameplay/BJ/WD_BJ.WD_BJ_C|GetSP1_Bet%20Amount _wd_bjhud_ref))
  (bind _sp2_bet_amount (Variables|/Game/Main/UI/Widgets/Gameplay/BJ/WD_BJ.WD_BJ_C|GetSP2_Bet%20Amount _wd_bjhud_ref))
  (bind _sp1_bet_amount_2 (Variables|/Game/Main/UI/Widgets/Gameplay/BJ/WD_BJ.WD_BJ_C|GetSP1_Bet%20Amount _wd_bjhud_ref_2))
  (bind _sp2_bet_amount_2 (Variables|/Game/Main/UI/Widgets/Gameplay/BJ/WD_BJ.WD_BJ_C|GetSP2_Bet%20Amount _wd_bjhud_ref_2))
  (Utilities|DMRefCheck
    (:Exec%20Out
      (if (Variables|/Game/Main/UI/Widgets/Gameplay/BJ/WD_BJ.WD_BJ_C|GetIsSplitted (Variables|/Game/Main/Blueprints/BP_DeckManager.BP_DeckManager_C|GetWD%20BJHUD%20Ref _dm_ref_2))
        (if (Variables|/Game/Main/Blueprints/BP_Blackjack.BP_Blackjack_C|GetSP1_IsDoubled _bj_ref_2)
          (switch Utilities|FlowControl|Switch|SwitchonE_Calc SP1_Calc
            (:NewEnumerator4
              (Utilities|MoneySum (* _sp1_bet_amount_2 2))
              (CallFunction|XPReward "NewEnumerator0" :!label _label))
            (:NewEnumerator7
              (CallFunction|XPReward "NewEnumerator1" :!label _label_2))
            (:NewEnumerator10
              (goto _label_2))
            (:NewEnumerator13
              (Utilities|MoneySum _sp1_bet_amount_2)
              (CallFunction|XPReward "NewEnumerator3" :!label _label_3)))
          (Default|ShowResults (Variables|/Game/Main/Blueprints/BP_DeckManager.BP_DeckManager_C|GetWD%20Results%20Ref (Variables|Default|GetDM%20ref)))
          (elif (Variables|/Game/Main/Blueprints/BP_Blackjack.BP_Blackjack_C|GetSP2_IsDoubled _bj_ref_2)
            (switch Utilities|FlowControl|Switch|SwitchonE_Calc SP2_Calc
              (:NewEnumerator5
                (Utilities|MoneySum (* _sp2_bet_amount_2 2))
                (goto _label))
              (:NewEnumerator8
                (goto _label_2))
              (:NewEnumerator11
                (goto _label_2))
              (:NewEnumerator14
                (Utilities|MoneySum _sp2_bet_amount_2)
                (goto _label_3)))
            (else
              (Utilities|FlowControl|Sequence
                (:then_0
                  (switch Utilities|FlowControl|Switch|SwitchonE_Calc SP1_Calc
                    (:NewEnumerator4
                      (Utilities|MoneySum (* _sp1_bet_amount 2))
                      (goto _label))
                    (:NewEnumerator7
                      _)
                    (:NewEnumerator10
                      _)
                    (:NewEnumerator13
                      (Utilities|MoneySum _sp1_bet_amount)
                      (goto _label_3))))
                (:then_1
                  (switch Utilities|FlowControl|Switch|SwitchonE_Calc SP2_Calc
                    (:NewEnumerator5
                      (Utilities|MoneySum (* _sp2_bet_amount 2))
                      (goto _label))
                    (:NewEnumerator8
                      _)
                    (:NewEnumerator11
                      _)
                    (:NewEnumerator14
                      (Utilities|MoneySum _sp2_bet_amount)
                      (goto _label_3)))))
              (if (Variables|/Game/Main/Blueprints/BP_Blackjack.BP_Blackjack_C|GetSP_Hand%20Done _bj_ref)
                (goto _label_3)
                (else
                  (Variables|/Game/Main/Blueprints/BP_Blackjack.BP_Blackjack_C|SetSP_Hand%20Done _bj_ref true))))))
        (elif (Variables|/Game/Main/Blueprints/BP_Blackjack.BP_Blackjack_C|GetIsDoubled _bj_ref_2)
          (switch Utilities|FlowControl|Switch|SwitchonE_Calc Calc
            (:NewEnumerator0
              (Utilities|MoneySum (* _betamount 2))
              (goto _label))
            (:NewEnumerator1
              (goto _label_2))
            (:NewEnumerator2
              (goto _label_2))
            (:NewEnumerator3
              (Utilities|MoneySum _betamount)
              (goto _label_3)))
          (else
            (switch Utilities|FlowControl|Switch|SwitchonE_Calc Calc
              (:NewEnumerator0
                (Utilities|MoneySum (* _betamount_2 2))
                (goto _label))
              (:NewEnumerator1
                (goto _label_2))
              (:NewEnumerator2
                (goto _label_2))
              (:NewEnumerator3
                (Utilities|MoneySum _betamount_2)
                (goto _label_3)))))))))

(fn XPReward
  (params (Result :type E_Result%20Enum :default "NewEnumerator0"))
  (Utilities|DMRefCheck
    (:Exec%20Out
      (switch Utilities|FlowControl|Switch|SwitchonE_Result Result
        (:NewEnumerator0
          (Utilities|ResultCheck
            (:Normal
              (Utilities|XPSum (Variables|Default|GetWin)
                (:Out%20Exec
                  _)))
            (:BJ
              (Utilities|XPSum (Variables|Default|GetBJWin)
                (:Out%20Exec
                  _)))
            (:2xBJ
              (Utilities|XPSum (Variables|Default|Get2xBJWin)
                (:Out%20Exec
                  _)))))
        (:NewEnumerator3
          (Utilities|ResultCheck
            (:Normal
              (Utilities|XPSum (Variables|Default|GetPush)
                (:Out%20Exec
                  _)))
            (:BJ
              (Utilities|XPSum (Variables|Default|GetBJPush)
                (:Out%20Exec
                  _)))
            (:2xBJ
              (Utilities|XPSum (Variables|Default|Get2xBJPush)
                (:Out%20Exec
                  (Variables|Default|SetWeFeelBad true))))))
        (:NewEnumerator1
          (Utilities|ResultCheck
            (:Normal
              (Utilities|XPSum (Variables|Default|GetLose)
                (:Out%20Exec
                  _))))))
      (return))))

(fn SettingBK
  (bind _returnvalue (SaveGame|DoesSaveGameExist "BK"))
  (if _returnvalue
    (bind _returnvalue_2 (SaveGame|LoadGamefromSlot "BK"))
    (bind _asbp_save_game (Utilities|Casting|CastToBP_SaveGame _returnvalue_2))
    (bind _output_get (Variables|Default|SetAs%20BP%20Save%20Game _asbp_save_game))
    (bind _isbk (Default|LoadBK _output_get))
    (Variables|Default|SetBankrupted _isbk)
    (else
      (bind _returnvalue_3 (SaveGame|CreateSaveGameObject "/Game/Main/MISC/BP_SaveGame.BP_SaveGame_C"))
      (SaveGame|SaveGametoSlot _returnvalue_3 "BK")
      (bind _returnvalue_4 (SaveGame|LoadGamefromSlot "BK"))
      (bind _asbp_save_game_2 (Utilities|Casting|CastToBP_SaveGame _returnvalue_4))
      (Variables|Default|SetAs%20BP%20Save%20Game _asbp_save_game_2))))