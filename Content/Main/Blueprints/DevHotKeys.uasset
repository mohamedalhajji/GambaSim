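; DevHotKeys is a developer cheat actor that grants money and XP.
; On BeginPlay it finds the BP_DeckManager in the level and caches it as DMRef.
; The DEV_Money and DEV_XP events each add a fixed amount directly to the matching value on the deck manager's StatsRef, with no validity checks.
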(event Custom|DEV_XP
  (bind _dm_ref (Variables|Default|GetDM%20Ref))
  (bind _stats_ref (Variables|/Game/Main/Blueprints/BP_DeckManager.BP_DeckManager_C|GetStats%20Ref _dm_ref))
  (Variables|/Game/Main/MISC/MyGameInstance.MyGameInstance_C|SetXP _stats_ref (+ (Variables|/Game/Main/MISC/MyGameInstance.MyGameInstance_C|GetXP _stats_ref) 1000)))

(event Custom|DEV_Money
  (bind _dm_ref (Variables|Default|GetDM%20Ref))
  (bind _stats_ref (Variables|/Game/Main/Blueprints/BP_DeckManager.BP_DeckManager_C|GetStats%20Ref _dm_ref))
  (Variables|/Game/Main/MISC/MyGameInstance.MyGameInstance_C|SetMoney _stats_ref (+ (Variables|/Game/Main/MISC/MyGameInstance.MyGameInstance_C|GetMoney _stats_ref) 1000)))

(event EventBeginPlay
  (bind _returnvalue (Actor|GetActorOfClass "/Game/Main/Blueprints/BP_DeckManager.BP_DeckManager_C"))
  (Variables|Default|SetDM%20Ref _returnvalue))

(fn ConstructionScript)