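; Blackjack game logic that runs a round: initial deal with hidden dealer card, hit, double, split and stand.
; DrawCard refills an empty deck, DeckTotalValue sums hands through a value map (ace reduction skips split hands), and TextToCard builds display strings from card names.
; On stand the dealer draws to 17, then CalculateWinner grades each hand.
; Outcome enums go to BP_StatsManager's Calc, and Reset clears hands and HUD flags.
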(event Custom|BJ_Split
  ;[0 0 0] Black Jack
  ;;[0.2 0 0] Switch Modes
  (Reusable|TexttoCard "NewEnumerator4")
  (if (Variables|Split|GetSP_IsAceSplit)
    (CallFunction|BJHit true "NewEnumerator4")))

(event Custom|BJ_Hit
  (params (Split :type Boolean) (Split%20Hand :type E_BJChoice%20Enum :default "NewEnumerator0"))
  ;[0 0 0] Black Jack
  ;;[0.2 0 0] Hit
  (Utilities|MoneyMGRRefChecker
    (:Exec%20Out
      (if Split
        (switch Utilities|FlowControl|Switch|SwitchonE_BJChoice Split%20Hand
          (:NewEnumerator4
            (Utilities|FlowControl|Sequence
              (:then_0
                (Reusable|DrawCard "NewEnumerator2" :!label _label)
                (Reusable|DeckTotalValue "NewEnumerator2")
                (if (> (Variables|Split|GetSP1_Total%20Value) 21)
                  (Variables|Split|SetSP1_Calc%20Var "NewEnumerator10")
                  (if (Variables|Split|GetSP_Hand%20Done)
                    (CallFunction|BJStand true))))
              (:then_1
                (Reusable|DrawCard "NewEnumerator3" :!label _label_2)
                (Reusable|DeckTotalValue "NewEnumerator3")
                (if (> (Variables|Split|GetSP2_Total%20Value) 21)
                  (Variables|Split|SetSP2_Calc%20Var "NewEnumerator11")
                  (if (Variables|Split|GetSP_Hand%20Done)
                    (CallFunction|BJStand true))))
              (:then_2
                (CallFunction|BJStand true))))
          (:NewEnumerator2
            (goto _label))
          (:NewEnumerator3
            (goto _label_2)))
        (else
          (Reusable|DrawCard "NewEnumerator0")
          (Reusable|DeckTotalValue "NewEnumerator0")
          (if (> (Variables|CardsInfo|GetPlayerTotalValue) 21)
            (Variables|MainVars|SetCalc%20Var "NewEnumerator2")
            (Default|Calc (Variables|Default|GetCalcMGR%20Ref) "NewEnumerator2" "NewEnumerator0" "NewEnumerator0")))))))

(event Custom|BJ_Stand
  (params (Split :type Boolean))
  (bind _dealertotalvalue (Variables|CardsInfo|GetDealerTotalValue))
  (bind _returnvalue (>= _dealertotalvalue 17))
  ;[0 0 0] Black Jack
  ;;[0.2 0 0] Stand
  (Variables|CardsInfo|SetDealerCardName (Utilities|String|Append (Variables|CardsInfo|GetDealerCardName) (Variables|CardsInfo|GetDealerSecretCards)))
  (Reusable|DeckTotalValue "NewEnumerator4")
  (if _returnvalue
    (Reusable|CalculateWinner Split)
    (else
      (while (not _returnvalue)
        (Reusable|DrawCard "NewEnumerator1")
        (Reusable|DeckTotalValue "NewEnumerator4"))
      (if (> (Variables|CardsInfo|GetDealerTotalValue) 21)
        (if Split
          (Reusable|CalculateWinner Split :!label _label)
          (else
            (Utilities|MoneyMGRRefChecker
              (:Exec%20Out
                (bind _output_get (Variables|MainVars|SetCalc%20Var "NewEnumerator0"))
                (Default|Calc (Variables|Default|GetCalcMGR%20Ref) _output_get "NewEnumerator0" "NewEnumerator0")))))
        (else
          (goto _label))))))

(event Custom|BJ_Double
  (params (Split :type Boolean) (Hand :type E_BJChoice%20Enum :default "NewEnumerator0"))
  ;[0 0 0] Black Jack
  ;;[0.2 0 0] Double
  (Utilities|MoneyMGRRefChecker
    (:Exec%20Out
      (if Split
        (switch Utilities|FlowControl|Switch|SwitchonE_BJChoice Hand
          (:NewEnumerator2
            (Variables|Split|SetSP1_IsDoubled true)
            (Reusable|DrawCard "NewEnumerator2")
            (Reusable|DeckTotalValue "NewEnumerator2")
            (if (> (Variables|Split|GetSP1_Total%20Value) 21)
              (Variables|Split|SetSP1_Calc%20Var "NewEnumerator10"))
            (if (Variables|Split|GetSP_Hand%20Done)
              (CallFunction|BJStand true)
              (else
                (Variables|Split|SetSP_Hand%20Done true))))
          (:NewEnumerator3
            (Variables|Split|SetSP2_IsDoubled true)
            (Reusable|DrawCard "NewEnumerator3")
            (Reusable|DeckTotalValue "NewEnumerator3")
            (if (> (Variables|Split|GetSP2_Total%20Value) 21)
              (Variables|Split|SetSP2_Calc%20Var "NewEnumerator11"))
            (if (Variables|Split|GetSP_Hand%20Done)
              (CallFunction|BJStand true)
              (else
                (Variables|Split|SetSP_Hand%20Done true)))))
        (else
          (Variables|MainVars|SetIsDoubled true)
          (Reusable|DrawCard "NewEnumerator0")
          (Reusable|DeckTotalValue "NewEnumerator0")
          (if (> (Variables|CardsInfo|GetPlayerTotalValue) 21)
            (bind _output_get (Variables|MainVars|SetCalc%20Var "NewEnumerator2"))
            (Default|Calc (Variables|Default|GetCalcMGR%20Ref) _output_get "NewEnumerator0" "NewEnumerator0")
            (else
              (CallFunction|BJStand false))))))))

(fn ConstructionScript
  (|CallParentFunction))

(fn DeckTotalValue
  (params (Hand :type E_BJChoice%20Enum :default "NewEnumerator0"))
  (bind _dealerhand (Variables|MainVars|GetDealerHand))
  (bind _player_s_ace_count (LocalVariables|GetPlayer's%20Ace%20Count))
  (bind _dealer_s_ace_count (LocalVariables|GetDealer's%20Ace%20Count))
  (bind _cardvaluemap (Variables|Default|GetCardValueMap))
  (bind _output (Utilities|Array|Get(acopy) _dealerhand))
  (bind _cardvalue (Utilities|Struct|BreakS_Cards _output))
  (bind _value (Utilities|Map|Find _cardvaluemap _cardvalue))
  (switch Utilities|FlowControl|Switch|SwitchonE_BJChoice Hand
    (:NewEnumerator0
      (Variables|CardsInfo|SetPlayerTotalValue 0)
      (for _array_element (Variables|MainVars|GetPlayerHand)
        (if (== (.Value (Utilities|Map|Find (Variables|Default|GetCardValueMap) (.CardValue (Utilities|Struct|BreakS_Cards _array_element)))) 11)
          (Math|Integer|IncrementInt (LocalVariables|GetPlayer's%20Ace%20Count)
            (:%20%20
              _)))
        (Variables|CardsInfo|SetPlayerTotalValue (+ (.Value (Utilities|Map|Find (Variables|Default|GetCardValueMap) (.CardValue (Utilities|Struct|BreakS_Cards _array_element)))) (Variables|CardsInfo|GetPlayerTotalValue)))
        (while (and (> (Variables|CardsInfo|GetPlayerTotalValue) 21) (> _player_s_ace_count 0))
          (Math|Integer|DecrementInt _player_s_ace_count
            (:%20%20
              (for _index (range _player_s_ace_count 0)
                (Variables|CardsInfo|SetPlayerTotalValue (- (Variables|CardsInfo|GetPlayerTotalValue) 10))))))))
    (:NewEnumerator1
      (if (== _value 11)
        (Math|Integer|IncrementInt (LocalVariables|GetDealer's%20Ace%20Count)
          (:%20%20
            _)))
      (Variables|CardsInfo|SetDealerTotalValue _value))
    (:NewEnumerator4
      (Variables|CardsInfo|SetDealerTotalValue 0)
      (for _array_element_2 (Variables|MainVars|GetDealerHand)
        (if (== (.Value (Utilities|Map|Find (Variables|Default|GetCardValueMap) (.CardValue (Utilities|Struct|BreakS_Cards _array_element_2)))) 11)
          (Math|Integer|IncrementInt (LocalVariables|GetDealer's%20Ace%20Count)
            (:%20%20
              _)))
        (Variables|CardsInfo|SetDealerTotalValue (+ (.Value (Utilities|Map|Find (Variables|Default|GetCardValueMap) (.CardValue (Utilities|Struct|BreakS_Cards _array_element_2)))) (Variables|CardsInfo|GetDealerTotalValue)))
        (while (and (> (Variables|CardsInfo|GetDealerTotalValue) 21) (> _dealer_s_ace_count 0))
          (Math|Integer|DecrementInt _dealer_s_ace_count
            (:%20%20
              (for _index_2 (range _dealer_s_ace_count 0)
                (Variables|CardsInfo|SetDealerTotalValue (- (Variables|CardsInfo|GetDealerTotalValue) 10))))))))
    (:NewEnumerator2
      (Variables|Split|SetSP1_Total%20Value 0)
      (for _array_element_3 (Variables|Split|GetSP1_PlayerHand)
        (Variables|Split|SetSP1_Total%20Value (+ (.Value (Utilities|Map|Find (Variables|Default|GetCardValueMap) (.CardValue (Utilities|Struct|BreakS_Cards _array_element_3)))) (Variables|Split|GetSP1_Total%20Value)))))
    (:NewEnumerator3
      (Variables|Split|SetSP2_Total%20Value 0)
      (for _array_element_4 (Variables|Split|GetSP2_PlayerHand)
        (Variables|Split|SetSP2_Total%20Value (+ (.Value (Utilities|Map|Find (Variables|Default|GetCardValueMap) (.CardValue (Utilities|Struct|BreakS_Cards _array_element_4)))) (Variables|Split|GetSP2_Total%20Value)))))))

(fn StartGame
  (params (ResetBet? :type Boolean))
  (Utilities|Reset ResetBet?
    (:ExecOut
      (CallFunction|InitializeCards)
      (Reusable|InitialDraws))))

(fn DrawCard
  (params (Deck :type E_BJChoice%20Enum :default "NewEnumerator0"))
  (if (> (Utilities|Array|Length (Variables|Default|GetDeck)) 0)
    _
    (else
      (CallFunction|InitializeCards)))
  (bind _output_get (Variables|CardsInfo|SetDrawnCard (Utilities|Array|Get(acopy) (Variables|Default|GetDeck))))
  (Utilities|Array|RemoveIndex (Variables|Default|GetDeck))
  (switch Utilities|FlowControl|Switch|SwitchonE_BJChoice Deck
    (:NewEnumerator0
      (Utilities|Array|Add (Variables|MainVars|GetPlayerHand) _output_get)
      (Reusable|TexttoCard "NewEnumerator0"))
    (:NewEnumerator1
      (Utilities|Array|Add (Variables|MainVars|GetDealerHand) _output_get)
      (Reusable|TexttoCard "NewEnumerator1"))
    (:NewEnumerator4
      (Utilities|Array|Add (Variables|MainVars|GetDealerHand) _output_get)
      (Variables|CardsInfo|SetDealerSecretCards (.Value (Utilities|Map|Find (Variables|Default|GetCardNameMap) _output_get))))
    (:NewEnumerator2
      (Utilities|Array|Add (Variables|Split|GetSP1_PlayerHand) _output_get)
      (Reusable|TexttoCard "NewEnumerator2"))
    (:NewEnumerator3
      (Utilities|Array|Add (Variables|Split|GetSP2_PlayerHand) _output_get)
      (Reusable|TexttoCard "NewEnumerator3")))
  (return))

(fn InitialDraws
  (bind _hand_1_check (LocalVariables|GetHand%201%20Check))
  (bind _hand_2_check (LocalVariables|GetHand%202%20Check))
  (Utilities|FlowControl|Sequence
    (:then_0
      (Reusable|DrawCard "NewEnumerator0" :!label _label) ; Player
      (Reusable|TexttoCard "NewEnumerator0")
      (Reusable|DeckTotalValue "NewEnumerator0")
      (Utilities|Array|Clear (LocalVariables|GetHand%201%20Check))
      (Utilities|Array|Clear (LocalVariables|GetHand%202%20Check))
      (for (_array_element _array_index) (Variables|MainVars|GetPlayerHand)
        (switch int _array_index
          (:0
            (Utilities|Array|Add _hand_1_check (.CardValue (Utilities|Struct|BreakS_Cards _array_element))))
          (:1
            (Utilities|Array|Add _hand_2_check (.CardValue (Utilities|Struct|BreakS_Cards _array_element))))))
      (if (Utilities|Array|Identical _hand_1_check _hand_2_check)
        (Variables|MainVars|SetEnableSplit true)))
    (:then_1
      (Reusable|DrawCard "NewEnumerator1") ; Dealer
      (Reusable|TexttoCard "NewEnumerator1")
      (Reusable|DeckTotalValue "NewEnumerator1"))
    (:then_2
      (goto _label))
    (:then_3
      (Reusable|DrawCard "NewEnumerator4")
      (Reusable|TexttoCard "NewEnumerator5"))))

(fn CalculateWinner
  (params (Split :type Boolean))
  (if Split
    (Utilities|FlowControl|Sequence
      (:then_0
        (bind (_bust _win _push _lose) (Reusable|ResultFormula (Variables|Split|GetSP1_Total%20Value)))
        (if _bust
          (Variables|Split|SetSP1_Calc%20Var "NewEnumerator10")
          (elif _win
            (Variables|Split|SetSP1_Calc%20Var "NewEnumerator4")
            (elif _push
              (Variables|Split|SetSP1_Calc%20Var "NewEnumerator13")
              (elif _lose
                (Variables|Split|SetSP1_Calc%20Var "NewEnumerator7"))))))
      (:then_1
        (bind (_bust_2 _win_2 _push_2 _lose_2) (Reusable|ResultFormula (Variables|Split|GetSP2_Total%20Value)))
        (if _bust_2
          (Variables|Split|SetSP2_Calc%20Var "NewEnumerator11")
          (elif _win_2
            (Variables|Split|SetSP2_Calc%20Var "NewEnumerator5")
            (elif _push_2
              (Variables|Split|SetSP2_Calc%20Var "NewEnumerator14")
              (elif _lose_2
                (Variables|Split|SetSP2_Calc%20Var "NewEnumerator8"))))))
      (:then_2
        (Default|Calc (Variables|Default|GetCalcMGR%20Ref) (Variables|MainVars|GetCalc%20Var) (Variables|Split|GetSP1_Calc%20Var) (Variables|Split|GetSP2_Calc%20Var) :!label _label)))
    (else
      (bind (_bust_3 _win_3 _push_3 _lose_3) (Reusable|ResultFormula (Variables|CardsInfo|GetPlayerTotalValue)))
      (if _bust_3
        (Variables|MainVars|SetCalc%20Var "NewEnumerator2")
        (goto _label)
        (elif _win_3
          (Variables|MainVars|SetCalc%20Var "NewEnumerator0")
          (goto _label)
          (elif _push_3
            (Variables|MainVars|SetCalc%20Var "NewEnumerator3")
            (goto _label)
            (elif _lose_3
              (Variables|MainVars|SetCalc%20Var "NewEnumerator1")
              (goto _label))))))))

(fn ResultFormula
  (params (Player's%20Deck :type Integer))
  (bind _dealertotalvalue (Variables|CardsInfo|GetDealerTotalValue))
  (if (> Player's%20Deck 21)
    (return true false false false)
    (else
      (if (> Player's%20Deck _dealertotalvalue)
        _
        (elif (== Player's%20Deck _dealertotalvalue)
          (return false false true false)
          (elif (and (> _dealertotalvalue Player's%20Deck) (<= _dealertotalvalue 21))
            (return false false false true)
            (else
              _))))
      (return false true false false))))

(fn TexttoCard
  (params (Player's%20Hand :type E_BJChoice%20Enum :default "NewEnumerator0"))
  (bind _playerhand (Variables|MainVars|GetPlayerHand))
  (bind _cardvaluemap (Variables|Default|GetCardValueMap))
  (bind _playerhand_2 (Variables|MainVars|GetPlayerHand))
  (bind _output (Utilities|Array|Get(acopy) _playerhand 1))
  (bind _output_2 (Utilities|Array|Get(acopy) _playerhand))
  (bind _output_3 (Utilities|Array|Get(acopy) _playerhand_2 1))
  (switch Utilities|FlowControl|Switch|SwitchonE_BJChoice Player's%20Hand
    (:NewEnumerator0
      (Variables|CardsInfo|SetPlayerCardName "")
      (for _array_element (Variables|MainVars|GetPlayerHand)
        (Variables|CardsInfo|SetPlayerCardName (Utilities|String|Append (Variables|CardsInfo|GetPlayerCardName) (.Value (Utilities|Map|Find (Variables|Default|GetCardNameMap) _array_element))))))
    (:NewEnumerator1
      (Variables|CardsInfo|SetDealerCardName "")
      (for _array_element_2 (Variables|MainVars|GetDealerHand)
        (Variables|CardsInfo|SetDealerCardName (Utilities|String|Append (Variables|CardsInfo|GetDealerCardName) (.Value (Utilities|Map|Find (Variables|Default|GetCardNameMap) _array_element_2)))))
      (Class|Widget|InvalidateLayoutandVolatility (Variables|Default|GetWD%20BJHUD%20Ref)))
    (:NewEnumerator4
      (Variables|Split|SetSP1_Total%20Value (.Value (Utilities|Map|Find _cardvaluemap (.CardValue (Utilities|Struct|BreakS_Cards (Utilities|Array|Get(acopy) _playerhand_2))))))
      (Variables|Split|SetSP2_Total%20Value (.Value (Utilities|Map|Find _cardvaluemap (.CardValue (Utilities|Struct|BreakS_Cards _output_3)))))
      (if (Utilities|Array|ContainsItem (Variables|Split|GetSP_AceCure) _output_3)
        (Variables|Split|SetSP_IsAceSplit true))
      (Variables|Split|SetSP1_PlayerHand (Utilities|Array|MakeArray _output_2))
      (Variables|Split|SetSP2_PlayerHand (Utilities|Array|MakeArray _output))
      (Variables|Split|SetSP1_CardT (Utilities|String|Append (Variables|Split|GetSP1_CardT) (.Value (Utilities|Map|Find (Variables|Default|GetCardNameMap) _output_2))))
      (Variables|Split|SetSP2_CardT (Utilities|String|Append (Variables|Split|GetSP2_CardT) (.Value (Utilities|Map|Find (Variables|Default|GetCardNameMap) _output)))))
    (:NewEnumerator2
      (Variables|Split|SetSP1_CardT "")
      (for _array_element_3 (Variables|Split|GetSP1_PlayerHand)
        (Variables|Split|SetSP1_CardT (Utilities|String|Append (Variables|Split|GetSP1_CardT) (.Value (Utilities|Map|Find (Variables|Default|GetCardNameMap) _array_element_3))))))
    (:NewEnumerator3
      (Variables|Split|SetSP2_CardT "")
      (for _array_element_4 (Variables|Split|GetSP2_PlayerHand)
        (Variables|Split|SetSP2_CardT (Utilities|String|Append (Variables|Split|GetSP2_CardT) (.Value (Utilities|Map|Find (Variables|Default|GetCardNameMap) _array_element_4))))))
    (:NewEnumerator5
      (Variables|CardsInfo|SetDealerCardName (Utilities|String|Append (.Value (Utilities|Map|Find (Variables|Default|GetCardNameMap) (Utilities|Array|Get(acopy) (Variables|MainVars|GetDealerHand)))) "?")))))