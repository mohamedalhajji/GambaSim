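; BP_MoneyManager settles blackjack bets, crediting the player's money for main-hand and two split-hand outcomes.
; Calc switches on the outcome, paying double the HUD's bet for wins, the bet for pushes and nothing for losses or busts.
; Processor adds and saves the amount through references on BP_DeckManager, which RefCheck re-acquires if invalid.
; Split outcomes also update HandVar to track settled hands before showing the results widget.
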(event EventBeginPlay
  (Utilities|FlowControl|Delay 0.2)
  (bind _returnvalue (Actor|GetActorOfClass "/Game/Main/Blueprints/BP_DeckManager.BP_DeckManager_C"))
  (Variables|Default|SetDM%20ref _returnvalue))

(fn ConstructionScript)

(fn Calc
  (params (Calc :type E_Calc%20Enum :default "NewEnumerator0"))
  (bind _dm_ref (Variables|Default|GetDM%20ref))
  (bind _wd_bjhud_ref (Variables|/Game/Main/Blueprints/BP_DeckManager.BP_DeckManager_C|GetWD%20BJHUD%20Ref _dm_ref))
  (bind _betamount (Variables|/Game/Main/UI/Widgets/Gameplay/BJ/BJHUD.BJHUD_C|GetBetAmount _wd_bjhud_ref))
  (bind _sp1_bet_amount (Variables|/Game/Main/UI/Widgets/Gameplay/BJ/BJHUD.BJHUD_C|GetSP1_Bet%20Amount _wd_bjhud_ref))
  (bind _sp2_bet_amount (Variables|/Game/Main/UI/Widgets/Gameplay/BJ/BJHUD.BJHUD_C|GetSP2_Bet%20Amount _wd_bjhud_ref))
  (Utilities|RefCheck
    (:Exec%20Out
      (bind _output_get (Variables|Default|SetCalc%20Var Calc))
      (switch Utilities|FlowControl|Switch|SwitchonE_Calc _output_get
        (:NewEnumerator0
          (Utilities|Processor (* _betamount 2)))
        (:NewEnumerator1
          _)
        (:NewEnumerator2
          _)
        (:NewEnumerator3
          (Utilities|Processor _betamount))
        (:NewEnumerator4
          (Utilities|Processor (* _sp1_bet_amount 2))
          (switch Utilities|FlowControl|Switch|SwitchonE_SP_Hand (Variables|Default|GetHand%20Var) :!label _label
            (:NewEnumerator0
              (Variables|Default|SetHand%20Var "NewEnumerator1"))
            (:NewEnumerator2
              (Variables|Default|SetHand%20Var "NewEnumerator3"))))
        (:NewEnumerator5
          (Utilities|Processor (* _sp2_bet_amount 2))
          (switch Utilities|FlowControl|Switch|SwitchonE_SP_Hand (Variables|Default|GetHand%20Var) :!label _label_2
            (:NewEnumerator0
              (Variables|Default|SetHand%20Var "NewEnumerator2"))
            (:NewEnumerator1
              (Variables|Default|SetHand%20Var "NewEnumerator3"))))
        (:NewEnumerator7
          (goto _label))
        (:NewEnumerator8
          (goto _label_2))
        (:NewEnumerator10
          (goto _label))
        (:NewEnumerator11
          (goto _label_2))
        (:NewEnumerator13
          (Utilities|Processor _sp1_bet_amount)
          (goto _label))
        (:NewEnumerator14
          (Utilities|Processor _sp2_bet_amount)
          (goto _label_2)))
      (Default|ShowResults (Variables|/Game/Main/Blueprints/BP_DeckManager.BP_DeckManager_C|GetWD%20Results%20Ref (Variables|Default|GetDM%20ref))))))