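; BP_SaveGame is a save object that stores the player's settings for audio, graphics and gameplay, plus a cheat flag.
; Each category has a Save function that copies its inputs into member variables and a Load function that returns them.
; It only holds values; it neither applies the settings nor writes to a save slot itself.
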(fn SaveAudio
  (params (Master :type Float%20%28double-precision%29) (SFX :type Float%20%28double-precision%29) (Music :type Float%20%28double-precision%29))
  (Variables|Default|SetMasterVol Master)
  (Variables|Default|SetSFXVol SFX)
  (Variables|Default|SetMusicVol Music))

(fn LoadAudio
  (return (Variables|Default|GetMasterVol) (Variables|Default|GetSFXVol) (Variables|Default|GetMusicVol)))

(fn SaveGraphics
  (params (Vsync :type Boolean) (Graphics :type Integer) (WMode :type EWindowMode%20Enum :default "Fullscreen") (DLSS :type Byte :default 0))
  (Variables|Default|SetSV_Vsync Vsync)
  (Variables|Default|SetSV_GraphicsIndex Graphics)
  (Variables|Default|SetSV_WindowMode WMode)
  (Variables|Default|SetSV_DLSS DLSS))

(fn LoadGraphics
  (return (Variables|Default|GetSV_Vsync) (Variables|Default|GetSV_GraphicsIndex) (Variables|Default|GetSV_WindowMode) (Variables|Default|GetSV_DLSS)))

(fn SaveGameplay
  (params (Sens :type Float%20%28double-precision%29))
  (Variables|Default|SetSV_Sens Sens))

(fn LoadGameplay
  (return (Variables|Default|GetSV_Sens)))

(fn SaveCheats
  (params (Cheat :type Boolean))
  (Variables|Default|SetSV_Cheated Cheat))

(fn LoadCheats
  (return (Variables|Default|GetSV_Cheated)))